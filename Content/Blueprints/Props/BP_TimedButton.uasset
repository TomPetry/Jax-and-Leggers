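; BP_TimedButton is a button prop that presses down quickly and rises back over a configurable activation time.
; LowerButton flags power as charging, turns the button's emissive green and moves it to its end position.
; While active, ElevateButton uses a DoOnce to move it back over ActivationTime, clearing the charging flag and glow.
; Calling ElevateButton while inactive resets that DoOnce.
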(event EventBeginPlay
  (|CallParentFunction) ; This node is disabled and will not be called.\nDrag off pins to build functionality.
)

(event Collision|EventActorBeginOverlap
  (params (OtherActor :type Actor%20Object%20Reference)))

(event EventTick
  (params (DeltaSeconds :type Float%20%28single-precision%29))
  (|CallParentFunction DeltaSeconds) ; This node is disabled and will not be called.\nDrag off pins to build functionality.
)

(event EventElevateButton
  (if (Variables|Default|GetIsActive)
    (Utilities|FlowControl|DoOnce false :!label _label
      (:Completed
        (Components|MoveComponentTo (Variables|Default|GetButton) (Variables|Default|GetButton_Start) "0, 0, 0" false false (Variables|Default|GetActivationTime) false)
        (Variables|Default|SetpwrIsCharging false)
        (Rendering|Material|SetVectorParameterValueonMaterials (Variables|Default|GetButton) "EmissiveColor" "0, 0, 0")))
    (else
      (goto _label Reset))))

(event EventLowerButton
  (Variables|Default|SetpwrIsCharging true)
  (Rendering|Material|SetVectorParameterValueonMaterials (Variables|Default|GetButton) "EmissiveColor" "0,0.800000, 0")
  (Components|MoveComponentTo (Variables|Default|GetButton) (Variables|Default|GetButton_End) "0, 0, 0" false false 0.1 false))

(fn ConstructionScript
  (|CallParentFunction))