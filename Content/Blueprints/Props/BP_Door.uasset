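; BP_Door is a two-panel sliding door that opens from activator states or its own SRActive flag.
; Each tick it polls BPI_Activatable actors, opening if every one in any activator set is active, or SRActive is true, otherwise closing.
; The SlideDoor timeline lerps both panels from cached start locations to fixed offsets and reverses to close.
; GetStatus exposes SRActive, while SetStatus forwards charging state to a powerline component.
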(event Custom|OpenDoor
  (bind _openmotion (Timeline|SlideDoor Play)
    (:Update
      (Transformation|SetRelativeLocation (Variables|Default|GetDoor_1) (Math|Vector|Lerp(Vector) (Variables|Default|GetDoor1_Start) "-50.000000, 0, 0" _openmotion) false false)
      (Transformation|SetRelativeLocation (Variables|Default|GetDoor_2) (Math|Vector|Lerp(Vector) (Variables|Default|GetDoor2_Start) "470.000000, 0, 0" _openmotion) false false))))

(event Custom|CloseDoor
  (bind _openmotion (Timeline|SlideDoor Reverse)
    (:Update
      (Transformation|SetRelativeLocation (Variables|Default|GetDoor_1) (Math|Vector|Lerp(Vector) (Variables|Default|GetDoor1_Start) "-50.000000, 0, 0" _openmotion) false false)
      (Transformation|SetRelativeLocation (Variables|Default|GetDoor_2) (Math|Vector|Lerp(Vector) (Variables|Default|GetDoor2_Start) "470.000000, 0, 0" _openmotion) false false))))

(event EventBeginPlay
  (Variables|Default|SetDoor1_Start (Variables|/Script/Engine.SceneComponent|GetRelativeLocation (Variables|Default|GetDoor_1)))
  (Variables|Default|SetDoor2_Start (Variables|/Script/Engine.SceneComponent|GetRelativeLocation (Variables|Default|GetDoor_2))))

(event Collision|EventActorBeginOverlap
  (params (OtherActor :type Actor%20Object%20Reference)))

(event EventTick
  (params (DeltaSeconds :type Float%20%28single-precision%29))
  (for _array_element (Variables|Default|GetActivators)
    (for _array_element_2 (.activatorset _array_element)
      (if (Utilities|DoesObjectImplementInterface _array_element_2 "/Game/Blueprints/Interfaces/BPI_Activatable.BPI_Activatable_C")
        (bind _isactive (Class|BPIActivatable|GetActiveStatus(Message) _array_element_2))
        (if (not _isactive)
          (Variables|Default|SetallActive false))))
    (if (Variables|Default|GetallActive)
      (Variables|Default|SetactiveSet true))
    (Variables|Default|SetallActive true))
  (if (or (Variables|Default|GetactiveSet) (Variables|Default|GetSRActive))
    (CallFunction|OpenDoor)
    (else
      (CallFunction|CloseDoor)))
  (Variables|Default|SetactiveSet false))

(fn ConstructionScript)

(fn GetStatus
  (params (param :type Boolean))
  (return (Variables|Default|GetSRActive)))

(fn SetStatus
  (params (isTrue :type Boolean) (PowerlineComponent :type Powerline%20Component%20Object%20Reference%20%28by%20ref%29))
  (Default|ChargePowerlineSR PowerlineComponent isTrue self)
  (return false))