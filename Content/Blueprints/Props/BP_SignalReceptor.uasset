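; BP_SignalReceptor is a prop that receives a boolean signal and toggles linked signal-activatable objects, passing each its powerline component.
; SetStatus triggers the toggle, and the receptor's actor tags pick the behavior.
; With both Green and Orange tags, the signal selects which of two targets flips while the other is forced off.
; Otherwise only the first target flips, after an interface check; the other status functions are stubs.
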(event Custom|Toggle
  (params (Green :type Boolean))
  (CallFunction|ToggleToggle Green))

(event Custom|ToggleToggle
  (params (Green :type Boolean))
  (bind _activatableone (Variables|Default|GetActivatableOne))
  (bind _activatabletwo (Variables|Default|GetActivatableTwo))
  (bind _activatableone_2 (Variables|Default|GetActivatableOne))
  (Development|PrintString (Utilities|String|ToString(Boolean) Green))
  (if (Utilities|Array|ContainsItem (Variables|Actor|GetTags self) "Green")
    (if (Utilities|Array|ContainsItem (Variables|Actor|GetTags self) "Orange")
      (if Green
        (bind _value (Class|BPISignalActivatable|GetStatus(Message) _activatableone_2 false))
        (Class|BPISignalActivatable|SetStatus(Message) _activatableone_2 (not _value) (Variables|Default|GetPowerlineComponent_One))
        (Class|BPISignalActivatable|SetStatus(Message) (Variables|Default|GetActivatableTwo) false (Variables|Default|GetPowerlineComponent_Two))
        (else
          (bind _value_2 (Class|BPISignalActivatable|GetStatus(Message) _activatabletwo false))
          (Class|BPISignalActivatable|SetStatus(Message) _activatabletwo (not _value_2) (Variables|Default|GetPowerlineComponent_Two))
          (Class|BPISignalActivatable|SetStatus(Message) (Variables|Default|GetActivatableOne) false (Variables|Default|GetPowerlineComponent_One))))
      (else
        (if (Utilities|DoesObjectImplementInterface _activatableone "/Game/Blueprints/Interfaces/BPI_SignalActivatable.BPI_SignalActivatable_C") :!label _label
          (bind _value_3 (Class|BPISignalActivatable|GetStatus(Message) _activatableone false))
          (Class|BPISignalActivatable|SetStatus(Message) _activatableone (not _value_3) (Variables|Default|GetPowerlineComponent_One)))))
    (else
      (goto _label))))

(fn ConstructionScript)

(fn GetActiveStatus
  (return false))

(fn GetStatus
  (return false))

(fn SetActiveStatus
  (params (isActive :type Boolean))
  (return false))

(fn SetStatus
  (params (Status :type Boolean))
  (CallFunction|Toggle Status)
  (return Status))