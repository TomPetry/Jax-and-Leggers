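; BP_SignalTester is a prop that tests signals by showing a sparks particle effect while its status is set on.
; SetStatus spawns a persistent sparks emitter above the actor when none exists, and destroys it when status is false.
; GetStatus and GetActiveStatus both return IsActive, which SetStatus never updates.
; The event graph and construction script hold no logic.
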(event EventBeginPlay)

(event Collision|EventActorBeginOverlap
  (params (OtherActor :type Actor%20Object%20Reference)))

(event EventTick
  (params (DeltaSeconds :type Float%20%28single-precision%29)))

(fn ConstructionScript)

(fn GetActiveStatus
  (return (Variables|Default|GetIsActive)))

(fn GetStatus
  (return (Variables|Default|GetIsActive)))

(fn SetStatus
  (params (Status :type Boolean))
  (if Status
    (Utilities|IsValid (Variables|Default|GetParticles)
      (:Is%20Valid
        _)
      (:Is%20Not%20Valid
        (bind _returnvalue (Effects|SpawnEmitteratLocation "/Game/StarterContent/Particles/P_Sparks.P_Sparks" (+ (Transformation|GetActorLocation) "0,0.000000,100.000000") "0, 0, 0" "1.000000,1.000000,1.000000" false))
        (Variables|Default|SetParticles _returnvalue)))
    (return false)
    (else
      (Utilities|IsValid (Variables|Default|GetParticles)
        (:Is%20Valid
          (Components|DestroyComponent (Variables|Default|GetParticles)))
        (:Is%20Not%20Valid
          (return false))))))