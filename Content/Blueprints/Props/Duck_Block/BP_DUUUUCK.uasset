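; BP_DUUUUCK is a duck block prop actor that can remove itself with a shrink animation.
; DestroyWithAnimation stores the current actor scale, multiplies it by the Shrink timeline's Scale track on each update, and destroys the actor when the timeline finishes.
; Tick only calls the parent, the construction script is empty, and leftover move and rotation nodes are never run.
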(event Custom|DestroyWithAnimation
  (bind _self self)
  (bind _output_get (Variables|Default|SetTempScale (Transformation|GetActorScale3D)))
  (bind _scale (Timeline|Shrink PlayFromStart)
    (:Update
      (Transformation|SetActorScale3D _self (* _output_get _scale)))
    (:Finished
      (Actor|DestroyActor _self))))

(event EventTick
  (params (DeltaSeconds :type Float%20%28single-precision%29))
  (|CallParentFunction DeltaSeconds))

(fn ConstructionScript)