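; BP_DuckBlockSpawner is a prop actor that spawns a series of BP_DBShowOff duck blocks at its own transform.
; Ten seconds after BeginPlay it sets a flag that lets Tick spawn blocks through a short repeating delay.
; A DoN node caps the number of spawns at the DuckAmounts value read from the GameInfoInstance game instance.
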(event Custom|SpawnDuckBlocks
  (Variables|Default|SetSpawnBlocks true))

(event EventBeginPlay
  (Utilities|FlowControl|Delay 1e+01)
  (CallFunction|SpawnDuckBlocks))

(event EventTick
  (params (DeltaSeconds :type Float%20%28single-precision%29))
  (if (Variables|Default|GetSpawnBlocks)
    (Utilities|FlowControl|Delay 0.4)
    (Utilities|FlowControl|DoN (Variables|/Game/Blueprints/AllLevels/GameInfoInstance.GameInfoInstance_C|GetDuckAmounts (.AsGame%20Info%20Instance (Utilities|Casting|CastToGameInfoInstance (Game|GetGameInstance))))
      (:Exit
        (Game|SpawnActorfromClass "/Game/Blueprints/Props/Duck_Block/BP_DBShowOff.BP_DBShowOff_C" (Transformation|GetActorTransform) "AdjustIfPossibleButAlwaysSpawn" 0 0)))))

(fn ConstructionScript)