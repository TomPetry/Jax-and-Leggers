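; Power receptor prop that draws connections from nearby charged BP_BatteryBlock actors to charge its powerline.
; Each tick it gathers overlapping batteries, then line-traces to each, establishing connections only when visible, charged and in range.
; Failed checks cut the connection, and blocked batteries leave the tracked array.
; The per-tick connection result drives PowerlineComponent, while the sphere's material color is set on or off as each battery is checked.
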(event Custom|CheckConnections
  (bind _self self)
  (bind _sphere (Variables|Default|GetSphere))
  ;[1 1 1] Loop through all nearby battery blocks
  (for _array_element (Variables|Default|GetConnectedActorArray)
    ;[1 1 1] Linetrace to battery block
    (bind _outhit (Collision|LineTraceByChannel (Transformation|GetActorLocation) (Transformation|GetActorLocation _array_element) "TraceTypeQuery1" false 0 "ForOneFrame"))
    ;[1 1 1] is the connection blocked by an obstacle?
    (if (and (.bblockinghit _outhit) (== (.hitactor _outhit) _array_element))
      ;[1 1 1] is the battery block in radius and charged?
      (bind _asbp_battery_block (Utilities|Casting|CastToBP_BatteryBlock _array_element))
      (if (and (> (Variables|/Game/Blueprints/Props/BP_BatteryBlock.BP_BatteryBlock_C|GetcurrentCharge _asbp_battery_block) 0.0) (< (.distance _outhit) (Variables|Default|GetOverlapRadius)))
        ;[1 1 1] Cut or Establish a Connection to the battery block
        (Default|EstablishConnection _asbp_battery_block _self)
        (Variables|Default|SetisConnected true)
        (Rendering|Material|SetVectorParameterValueonMaterials _sphere "Color" (Math|Conversions|ToVector(LinearColor) (Variables|Default|GetON_Color)))
        (else
          (Default|DeleteConnection _asbp_battery_block _self)
          (Rendering|Material|SetVectorParameterValueonMaterials _sphere "Color" (Math|Conversions|ToVector(LinearColor) (Variables|Default|GetOFF_Color)))))
      (else
        ;[1 1 1] Cut the connection to the battery block that is not "in sight"
        (bind _asbp_battery_block_2 (Utilities|Casting|CastToBP_BatteryBlock _array_element))
        (Default|DeleteConnection _asbp_battery_block_2 self)
        (Utilities|Array|RemoveItem (Variables|Default|GetConnectedActorArray) _array_element)
        (Rendering|Material|SetVectorParameterValueonMaterials (Variables|Default|GetSphere) "Color" (Math|Conversions|ToVector(LinearColor) (Variables|Default|GetOFF_Color))))))
  (bind _output_get (Variables|Default|SetPwrIsCharging (Variables|Default|GetisConnected)))
  (Default|ChargePowerline (Variables|Default|GetPowerlineComponent) _output_get)
  (Variables|Default|SetisConnected false))

(event EventTick
  (params (DeltaSeconds :type Float%20%28single-precision%29))
  (CallFunction|CheckConnections)
  ;[1 1 1] Get all battery blocks within range and store them in an array
  (bind (_outactors _returnvalue) (Collision|SphereOverlapActors (Transformation|GetWorldLocation (Variables|Default|GetSphere)) (Variables|Default|GetOverlapRadius) (Utilities|Array|MakeArray "ObjectTypeQuery2") "/Game/Blueprints/Props/BP_BatteryBlock.BP_BatteryBlock_C"))
  (if _returnvalue
    (for _array_element _outactors
      (Utilities|Array|AddUnique (Variables|Default|GetConnectedActorArray) _array_element))))

(fn ConstructionScript
  (Rendering|Material|SetVectorParameterValueonMaterials (Variables|Default|GetSphere) "Color" (Math|Conversions|ToVector(LinearColor) (Variables|Default|GetOFF_Color))))

(fn GetActiveStatus
  (return (Variables|Default|GetisActivated)))

(fn SetActiveStatus
  (params (isActive :type Boolean))
  (bind _output_get (Variables|Default|SetisActivated isActive))
  (return _output_get))