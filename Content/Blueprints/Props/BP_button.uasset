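; Pressure button prop that powers a powerline while enough actors overlap its trigger, optionally restricted to Jax or Leggers.
; The construction script uses Access to set the class filter, button material and overlap threshold, which is higher for the unfiltered Both mode.
; Tick polls overlaps, lowers or raises the button, toggles its green emissive and passes the charging state to PowerlineComponent1.
; An IsActive getter and setter exist but do not gate this logic.
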(event Custom|LowerButton
  (Variables|Powerline|SetpwrIsCharging true)
  (Rendering|Material|SetVectorParameterValueonMaterials (Variables|Default|GetButton) "EmissiveColor" "0,0.800000, 0")
  (Components|MoveComponentTo (Variables|Default|GetButton) (Variables|Button|GetButton_End) "0, 0, 0" false false 0.1 false))

(event Custom|ElevateButton
  (Variables|Powerline|SetpwrIsCharging false)
  (Rendering|Material|SetVectorParameterValueonMaterials (Variables|Default|GetButton) "EmissiveColor" "0, 0, 0")
  (Components|MoveComponentTo (Variables|Default|GetButton) (Variables|Button|GetButton_Start) "0, 0, 0" false false 0.1 false))

(event EventBeginPlay
  (Variables|Button|SetButton_Start (Variables|/Script/Engine.SceneComponent|GetRelativeLocation (Variables|Default|GetButton))))

(event EventTick
  (params (DeltaSeconds :type Float%20%28single-precision%29))
  (if (> (Utilities|Array|Length (Collision|GetOverlappingActors (Variables|Default|GetButtonTrigger) (Variables|Button|GetClassReference) :!class /Script/Engine.PrimitiveComponent)) (Variables|Button|GetOverlappingActorStart))
    (CallFunction|LowerButton)
    (else
      (CallFunction|ElevateButton)))
  (Default|ChargePowerline (Variables|Default|GetPowerlineComponent1) (Variables|Powerline|GetpwrIsCharging)))

(fn ConstructionScript
  (bind _button (Variables|Default|GetButton))
  (switch Utilities|FlowControl|Switch|SwitchonAccessEnum (Variables|Button|GetAccess)
    (:NewEnumerator0
      (Variables|Button|SetClassReference 0)
      (Rendering|Material|SetMaterial _button 0 "/Game/StarterContent/Materials/M_Wood_Oak.M_Wood_Oak")
      (Variables|Button|SetOverlappingActorStart 1))
    (:NewEnumerator1
      (Variables|Button|SetClassReference "/Game/Blueprints/Characters/Jax.Jax_C")
      (Rendering|Material|SetMaterial _button 0 "/Game/Blueprints/Materials/M_TimedButton_Jax.M_TimedButton_Jax")
      (Variables|Button|SetOverlappingActorStart 0 :!label _label))
    (:NewEnumerator2
      (Variables|Button|SetClassReference "/Game/Blueprints/Characters/Leggers.Leggers_C")
      (Rendering|Material|SetMaterial _button 0 "/Game/Blueprints/Materials/M_TimedButton_Leggers.M_TimedButton_Leggers")
      (goto _label))))

(fn GetActiveStatus
  (return (Variables|Button|GetIsActive)))

(fn SetActiveStatus
  (params (isActive :type Boolean))
  (bind _output_get (Variables|Button|SetIsActive isActive))
  (return _output_get))