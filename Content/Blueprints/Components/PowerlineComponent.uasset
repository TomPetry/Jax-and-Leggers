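; Actor component that lights a chain of powerline decals to show power charging toward an activatable owner.
; On BeginPlay it finds BP_Powerline actors tagged with the owner's object name, colors them off and splits the total activation time evenly among them.
; Repeated ChargePowerline calls step decals on or off by delta time, setting the owner active only when fully lit.
; ChargePowerline_SR mirrors this, setting SRActive on a passed door instead.
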(event Custom|ChargePowerline_SR
  (params (pwrIsCharging :type Boolean) (Door :type BP%20Door%20Object%20Reference%20%28by%20ref%29))
  (bind _powerlinedecals (Variables|Default|GetPowerlineDecals))
  (bind _returnvalue (Utilities|Array|Length _powerlinedecals))
  (Variables|ChargePowerline_SR|SetSRDoor Door)
  (if (and (Variables|Default|GetisActivatable) (== (Utilities|Array|Length (Variables|Default|GetPowerlineDecals)) 0))
    (Variables|/Game/Blueprints/Props/BP_Door.BP_Door_C|SetSRActive (Variables|ChargePowerline_SR|GetSRDoor) pwrIsCharging)
    (elif pwrIsCharging
      (if (== (Variables|Default|GetCurrentDecalIndex) -1)
        (Variables|Default|SetCurrentDecalIndex 0))
      (if (< (Variables|Default|GetCurrentDecalIndex) (Utilities|Array|Length (Variables|Default|GetPowerlineDecals)))
        (if (Variables|/Game/Blueprints/Props/BP_Powerline.BP_Powerline_C|GetisActive (Utilities|Array|Get(acopy) (Variables|Default|GetPowerlineDecals) (Variables|Default|GetCurrentDecalIndex)))
          (Math|Integer|IncrementInt (Variables|Default|GetCurrentDecalIndex) :!label _label)
          (elif (<= (Variables|Default|GetCurrentTime) 0.0)
            (Rendering|Material|SetVectorParameterValue (Variables|/Game/Blueprints/Props/BP_Powerline.BP_Powerline_C|GetMaterialInstance (Utilities|Array|Get(acopy) (Variables|Default|GetPowerlineDecals) (Variables|Default|GetCurrentDecalIndex))) "Color" (Variables|Default|GetON_Color) :!class /Script/Engine.MaterialInstanceDynamic)
            (Variables|/Game/Blueprints/Props/BP_Powerline.BP_Powerline_C|SetisActive (Utilities|Array|Get(acopy) (Variables|Default|GetPowerlineDecals) (Variables|Default|GetCurrentDecalIndex)) true)
            (Variables|Default|SetCurrentTime (Variables|Default|GetMaxIntervalTime))
            (goto _label)
            (else
              (Variables|Default|SetCurrentTime (- (Variables|Default|GetCurrentTime) (Utilities|Time|GetWorldDeltaSeconds))))))
        (else
          (Variables|/Game/Blueprints/Props/BP_Door.BP_Door_C|SetSRActive (Variables|ChargePowerline_SR|GetSRDoor) true)))
      (else
        (if (== (Variables|Default|GetCurrentDecalIndex) _returnvalue)
          (Variables|Default|SetCurrentDecalIndex (- _returnvalue 1)))
        (if (>= (Variables|Default|GetCurrentDecalIndex) 0)
          (Variables|/Game/Blueprints/Props/BP_Door.BP_Door_C|SetSRActive (Variables|ChargePowerline_SR|GetSRDoor) false)
          (if (Variables|/Game/Blueprints/Props/BP_Powerline.BP_Powerline_C|GetisActive (Utilities|Array|Get(acopy) (Variables|Default|GetPowerlineDecals) (Variables|Default|GetCurrentDecalIndex)))
            (if (<= (Variables|Default|GetCurrentTime) 0.0)
              (Rendering|Material|SetVectorParameterValue (Variables|/Game/Blueprints/Props/BP_Powerline.BP_Powerline_C|GetMaterialInstance (Utilities|Array|Get(acopy) (Variables|Default|GetPowerlineDecals) (Variables|Default|GetCurrentDecalIndex))) "Color" (Variables|Default|GetOFF_Color) :!class /Script/Engine.MaterialInstanceDynamic)
              (Variables|/Game/Blueprints/Props/BP_Powerline.BP_Powerline_C|SetisActive (Utilities|Array|Get(acopy) (Variables|Default|GetPowerlineDecals) (Variables|Default|GetCurrentDecalIndex)) false)
              (Variables|Default|SetCurrentTime (Variables|Default|GetMaxIntervalTime))
              (Math|Integer|DecrementInt (Variables|Default|GetCurrentDecalIndex) :!label _label_2)
              (else
                (Variables|Default|SetCurrentTime (- (Variables|Default|GetCurrentTime) (Utilities|Time|GetWorldDeltaSeconds)))))
            (else
              (goto _label_2))))))))

(event Custom|InitPowerline
  (if (Utilities|DoesObjectImplementInterface (Variables|Default|GetOwner) "/Game/Blueprints/Interfaces/BPI_Activatable.BPI_Activatable_C")
    (Variables|Default|SetisActivatable true)
    (switch Utilities|FlowControl|Switch|SwitchonPowerlineColorEnum (Variables|Default|GetPwrColorMode)
      (:NewEnumerator0
        (Variables|Default|SetOFF_Color "(R=0.000000,G=0.000000,B=1.000000,A=1.000000)")
        (Variables|Default|SetON_Color "(R=1.000000,G=0.000000,B=0.000000,A=1.000000)"))
      (:NewEnumerator1
        (Variables|Default|SetOFF_Color "(R=1.000000,G=0.272000,B=0.000000,A=1.000000)")
        (Variables|Default|SetON_Color "(R=0.000000,G=1.000000,B=0.000000,A=1.000000)")))
    (bind _outactors (Actor|GetAllActorswithTag (Utilities|String|StringToName (Utilities|GetObjectName (Variables|Default|GetOwner)))))
    (for _array_element _outactors
      (bind _asbp_powerline (Utilities|Casting|CastToBP_Powerline _array_element))
      (Rendering|Material|SetVectorParameterValue (Variables|/Game/Blueprints/Props/BP_Powerline.BP_Powerline_C|GetMaterialInstance _asbp_powerline) "Color" (Variables|Default|GetOFF_Color) :!class /Script/Engine.MaterialInstanceDynamic)
      (Utilities|Array|Add (Variables|Default|GetPowerlineDecals) _asbp_powerline)
      (bind _output_get (Variables|Default|SetMaxIntervalTime (/ (Variables|Default|GetMaxActivationTime) (Math|Conversions|ToFloat(Integer) (Utilities|Array|Length (Variables|Default|GetPowerlineDecals))))))
      (Variables|Default|SetCurrentTime _output_get))))

(event Custom|ChargePowerline
  (params (pwrIsCharging :type Boolean))
  (bind _powerlinedecals (Variables|Default|GetPowerlineDecals))
  (bind _returnvalue (Utilities|Array|Length _powerlinedecals))
  (if (and (Variables|Default|GetisActivatable) (== (Utilities|Array|Length (Variables|Default|GetPowerlineDecals)) 0))
    (Class|BPIActivatable|SetActiveStatus(Message) (Variables|Default|GetOwner) pwrIsCharging)
    (elif pwrIsCharging
      (if (== (Variables|Default|GetCurrentDecalIndex) -1)
        (Variables|Default|SetCurrentDecalIndex 0))
      (if (< (Variables|Default|GetCurrentDecalIndex) (Utilities|Array|Length (Variables|Default|GetPowerlineDecals)))
        (if (Variables|/Game/Blueprints/Props/BP_Powerline.BP_Powerline_C|GetisActive (Utilities|Array|Get(acopy) (Variables|Default|GetPowerlineDecals) (Variables|Default|GetCurrentDecalIndex)))
          (Math|Integer|IncrementInt (Variables|Default|GetCurrentDecalIndex) :!label _label)
          (elif (<= (Variables|Default|GetCurrentTime) 0.0)
            (Rendering|Material|SetVectorParameterValue (Variables|/Game/Blueprints/Props/BP_Powerline.BP_Powerline_C|GetMaterialInstance (Utilities|Array|Get(acopy) (Variables|Default|GetPowerlineDecals) (Variables|Default|GetCurrentDecalIndex))) "Color" (Variables|Default|GetON_Color) :!class /Script/Engine.MaterialInstanceDynamic)
            (Variables|/Game/Blueprints/Props/BP_Powerline.BP_Powerline_C|SetisActive (Utilities|Array|Get(acopy) (Variables|Default|GetPowerlineDecals) (Variables|Default|GetCurrentDecalIndex)) true)
            (Variables|Default|SetCurrentTime (Variables|Default|GetMaxIntervalTime))
            (goto _label)
            (else
              (Variables|Default|SetCurrentTime (- (Variables|Default|GetCurrentTime) (Utilities|Time|GetWorldDeltaSeconds))))))
        (else
          (Class|BPIActivatable|SetActiveStatus(Message) (Variables|Default|GetOwner) true)))
      (else
        (if (== (Variables|Default|GetCurrentDecalIndex) _returnvalue)
          (Variables|Default|SetCurrentDecalIndex (- _returnvalue 1)))
        (if (>= (Variables|Default|GetCurrentDecalIndex) 0)
          (Class|BPIActivatable|SetActiveStatus(Message) (Variables|Default|GetOwner) false)
          (if (Variables|/Game/Blueprints/Props/BP_Powerline.BP_Powerline_C|GetisActive (Utilities|Array|Get(acopy) (Variables|Default|GetPowerlineDecals) (Variables|Default|GetCurrentDecalIndex)))
            (if (<= (Variables|Default|GetCurrentTime) 0.0)
              (Rendering|Material|SetVectorParameterValue (Variables|/Game/Blueprints/Props/BP_Powerline.BP_Powerline_C|GetMaterialInstance (Utilities|Array|Get(acopy) (Variables|Default|GetPowerlineDecals) (Variables|Default|GetCurrentDecalIndex))) "Color" (Variables|Default|GetOFF_Color) :!class /Script/Engine.MaterialInstanceDynamic)
              (Variables|/Game/Blueprints/Props/BP_Powerline.BP_Powerline_C|SetisActive (Utilities|Array|Get(acopy) (Variables|Default|GetPowerlineDecals) (Variables|Default|GetCurrentDecalIndex)) false)
              (Variables|Default|SetCurrentTime (Variables|Default|GetMaxIntervalTime))
              (Math|Integer|DecrementInt (Variables|Default|GetCurrentDecalIndex) :!label _label_2)
              (else
                (Variables|Default|SetCurrentTime (- (Variables|Default|GetCurrentTime) (Utilities|Time|GetWorldDeltaSeconds)))))
            (else
              (goto _label_2))))))))

(event EventTick
  (params (DeltaSeconds :type Float%20%28single-precision%29)))

(event EventBeginPlay
  (Variables|Default|SetOwner (Components|GetOwner))
  (CallFunction|InitPowerline))